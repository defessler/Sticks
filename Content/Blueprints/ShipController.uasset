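; ShipController is a player controller for ship characters that tracks kills and deaths and shows the ShipHUD widget.
; BeginPlay zeroes the score and adds the HUD to the viewport, and separate events add a delta to each counter.
; Respawn runs only with authority, spawning a new ShipCharacter at a randomly chosen PlayerStart and possessing it.
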(event Custom|Respawn
  ;[1 1 1] Restart at a random start point.
  (Networking|SwitchHasAuthority
    (:Authority
      (bind _outactors (Actor|GetAllActorsOfClass "/Script/Engine.PlayerStart"))
      (bind _returnvalue (Game|SpawnActorfromClass "/Game/Blueprints/ShipCharacter.ShipCharacter_C" (Transformation|GetActorTransform (Utilities|Array|Get(acopy) _outactors (Math|Random|RandomInteger (Utilities|Array|Length _outactors)))) true 0 0))
      (Pawn|Possess _returnvalue))))

(event Custom|IncrementDeaths
  (params (Delta :type Integer))
  ;[1 1 1] Handle Score
  (Variables|Default|SetDeaths (+ Delta (Variables|Default|GetDeaths))))

(event Custom|IncrementKills
  (params (Delta :type Integer))
  ;[1 1 1] Handle Score
  (Variables|Default|SetKills (+ Delta (Variables|Default|GetKills))))

(event EventBeginPlay
  ;[1 1 1] Reset score and add HUD.
  (Variables|Default|SetKills 0)
  (Variables|Default|SetDeaths 0)
  (bind _returnvalue (UserInterface|CreateWidget "/Game/Blueprints/ShipHUD.ShipHUD_C"))
  (UserInterface|Viewport|AddtoViewport _returnvalue 0))

(fn ConstructionScript)