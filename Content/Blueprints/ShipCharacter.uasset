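; Player-controlled ship character for a multiplayer shooter, with axis-driven movement and rotation toward the cursor.
; Trigger input runs through the server to fire twin lasers on all clients, using a looping timer with a DoOnce reset to cap fire rate.
; Tick refreshes the health bar widget.
; Damage resolves on authority; death increments the controller's count, hides the ship with an explosion, then respawns and destroys it after a delay.
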(event Custom|Fire
  ;[1 1 1] Spawns projectiles on server and all clients.
  (Game|SpawnActorfromClass "/Game/Blueprints/Laser.Laser_C" (Transformation|GetWorldTransform (Variables|Default|GetGunLeft)) false 0 0)
  (Game|SpawnActorfromClass "/Game/Blueprints/Laser.Laser_C" (Transformation|GetWorldTransform (Variables|Default|GetGunRight)) false 0 0)
  (Class|GameplayStatics|PlaySoundAttached "/Game/Audio/LaserFire.LaserFire" (Variables|Default|GetShipMesh)))

(event Custom|DeathSequence
  ;[1 1 1] Server tells clients to set up death squence by hiding mesh and spawning explosion.
  (Input|DisableInput 0)
  (CallFunction|ReleaseTrigger)
  (Collision|SetCollisionResponsetoChannel (Variables|Default|GetCapsuleComponent) "ECC_WorldDynamic" "ECR_Ignore")
  (Rendering|SetVisibility (Variables|Default|GetShipMesh) false true)
  (Game|SpawnActorfromClass "/Game/Blueprints/Explosion.Explosion_C" (Transformation|GetActorTransform) false 0 0))

(event Custom|ReleaseTrigger
  ;[1 1 1] Server calls Fire on clients on a timer.
  (Utilities|Time|ClearTimerbyFunctionName 0 "Fire"))

(event Custom|PullTrigger
  (bind _dps (Variables|Default|GetDPS))
  (bind _returnvalue (/ 1.0 _dps))
  ;[1 1 1] Server calls Fire on clients on a timer.
  (Utilities|FlowControl|DoOnce false
    (:Completed
      (CallFunction|Fire)
      (Utilities|Time|SetTimerbyFunctionName 0 "Fire" _returnvalue true)
      (Utilities|Time|SetTimerbyFunctionName 0 "ResetFireTimer" _returnvalue))))

(event Custom|ResetFireTimer
  (bind _dps (Variables|Default|GetDPS))
  (bind _returnvalue (/ 1.0 _dps))
  ;[1 1 1] Server calls Fire on clients on a timer.
  (Utilities|FlowControl|DoOnce false) ; enters at Reset
)

(event EventTick
  (params (DeltaSeconds :type Float%20%28single-precision%29))
  ;[1 1 1] Set rotation based on mouse position.
  (CallFunction|SetRotation)
  (Utilities|FlowControl|Delay 0.1) ; Small delay to help performance.
  (bind _ashealth_bar (Utilities|Casting|CastToHealthBar (UserInterface|GetUserWidgetObject (Variables|Default|GetHealthBar))))
  (Default|SetHealthBar _ashealth_bar (Variables|Default|GetHealth)))

(event EventAffectHealth
  (params (Delta :type Float%20%28single-precision%29) (Attacker :type Pawn%20Object%20Reference))
  ;[1 1 1] Handle health and respawning.
  (Networking|SwitchHasAuthority
    (:Authority
      (Class|BaseCharacter|CalculateHealth Delta)
      (if (Variables|Default|GetisDead)
        (bind _asship_controller (Utilities|Casting|CastToShipController (Pawn|GetController)))
        (Default|IncrementDeaths _asship_controller 1)
        (CallFunction|DeathSequence)
        (Utilities|FlowControl|Delay 3.0)
        (bind _asship_controller_2 (Utilities|Casting|CastToShipController (Pawn|GetController)))
        (Default|Respawn _asship_controller_2)
        (Actor|DestroyActor)))))

(event Input|ActionEvents|InputActionPrimaryFire
  ;[1 1 1] Client calls PullTrigger/ReleaseTrigger on server.
  (:Pressed
    (CallFunction|PullTrigger))
  (:Released
    (CallFunction|ReleaseTrigger)))

(event Input|AxisEvents|InputAxisMoveX
  (params (AxisValue :type Float%20%28single-precision%29))
  ;[1 1 1] Set WASD movement.
  (Pawn|Input|AddMovementInput "1.000000, 0, 0" AxisValue false))

(event Input|AxisEvents|InputAxisMoveY
  (params (AxisValue :type Float%20%28single-precision%29))
  ;[1 1 1] Set WASD movement.
  (Pawn|Input|AddMovementInput "0,1.000000, 0" AxisValue false))

(fn ConstructionScript)

(fn SetRotation
  ;[1 1 1] Set rotation based on mouse position.
  (if (not (Variables|Default|GetisDead))
    (bind _asplayer_controller (Utilities|Casting|CastToPlayerController (Pawn|GetController))
      (:then
        (Pawn|SetControlRotation _asplayer_controller (Math|Rotator|FindLookatRotation (Transformation|GetActorLocation) (.location (.HitResult (Game|Player|GetHitResultUnderCursorbyChannel _asplayer_controller "TraceTypeQuery2" false))))))
      (:CastFailed
        _)))
  (return))