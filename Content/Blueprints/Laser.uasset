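; Laser projectile actor that damages IDamagable actors it overlaps, ignoring its own Instigator.
; On a valid hit it spawns sparks and sends a negative health delta of half its Damage through AffectHealthMessage.
; For ShipCharacter targets only, it credits a kill to the Instigator's ShipController if the target is dead, then plays a sound and destroys itself.
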(event Collision|EventActorBeginOverlap
  (params (OtherActor :type Actor%20Object%20Reference))
  (bind _instigator (Variables|Actor|GetInstigator))
  (if (!= _instigator OtherActor)
    (if (Utilities|DoesObjectImplementInterface OtherActor "/Game/Blueprints/iDamagable.iDamagable_C")
      (Effects|SpawnEmitteratLocation "/Game/Particles/LaserSparks.LaserSparks" (Transformation|GetActorLocation))
      (Class|IDamagable|AffectHealth(Message) OtherActor (/ (Variables|Default|GetDamage) -2.0) _instigator)
      (bind _asship_character (Utilities|Casting|CastToShipCharacter OtherActor))
      (if (Variables|/Script/Sticks.BaseCharacter|GetisDead _asship_character)
        (bind _asship_controller (Utilities|Casting|CastToShipController (Pawn|GetController _instigator))
          (:then
            (Default|IncrementKills _asship_controller 1))
          (:CastFailed
            _)))
      (Class|GameplayStatics|PlaySoundAttached "/Game/Audio/TemplateTSS_WeaponFire.TemplateTSS_WeaponFire" (Variables|Default|GetLaserMesh))
      (Actor|DestroyActor))))

(fn ConstructionScript)